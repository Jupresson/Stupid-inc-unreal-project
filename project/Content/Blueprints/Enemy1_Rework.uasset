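; Enemy AI that loops a move request intended for random wandering and fires bullets when it perceives the player.
; BeginPlay starts movement, adds AI perception and calls GunFire once; perceiving BF_FPS_Character sets CanSeePlayer and fires again.
; GunFire spawns a Bullet, halts movement and recurses without delay while CanSeePlayer, which is never cleared here.
; Its timer targets an empty ShootPlayer function, and the perception-side clear misspells that name.
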(event `MoveRandomly`
  ; Movement
  (`|AIMoveTo` null (0.0 0.0 0.0) null
    (:`then`
      (`NavigationSystemV1.K2_GetRandomLocationInNavigableRadius` (`self.K2_GetActorLocation`) 300.0 null null))
    (:`OnSuccess`
      (`KismetSystemLibrary.PrintString` "MoveSuccess")
      (`self.MoveRandomly`))
    (:`OnFail`
      (`KismetSystemLibrary.PrintString` "MoveFail"))))

(event `self.ReceiveBeginPlay`
  ; Movement
  (`self.MoveRandomly`)
  (bind _returnvalue (`AddComponent|NODE_AddAIPerceptionComponent-2`))
  (add `AIPerceptionComponent.OnPerceptionUpdated` _returnvalue (delegate `OnPerceptionUpdated_Event`))
  (`self.GunFire` self (0.0 0.0 0.0)))

(event `OnPerceptionUpdated_Event`
  (params (UpdatedActors :type "Array of Actor Object Reference (by ref)"))
  ; Movement
  (for _array_element UpdatedActors
    (cast `/Game/Blueprints/BF_FPS_Character` _array_element
      (:`then`
        (set `self.canSeePlayer?` true)
        (`self.GunFire` (0.0 0.0 0.0)))
      (:`CastFailed`
        (`KismetSystemLibrary.K2_ClearTimer` null "Shoot Player")))))

(event `GunFire`
  (params (Start :type "Vector Structure (by ref)"))
  ; Gun Fire
  (`self.ShootPlayer`)
  (`|SpawnActorFromClass` "/Game/Blueprints/Bullet.Bullet_C" (`self.GetTransform`) "Undefined" "MultiplyWithRoot" null null)
  (`MovementComponent.StopMovementImmediately` (`self.CharacterMovement`))
  (`KismetSystemLibrary.K2_SetTimer` null "ShootPlayer" 2.0)
  (if (`self.canSeePlayer?`)
    (`self.GunFire` (0.0 0.0 0.0))
    (else
      (`KismetSystemLibrary.K2_ClearTimer` null "ShootPlayer"))))

(fn `ShootPlayer`)

(fn `UserConstructionScript`)