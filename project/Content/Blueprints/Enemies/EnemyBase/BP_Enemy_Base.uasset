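; Base melee enemy character that attacks the player when nearby, with its AI controller handling state.
; Tick switches the controller to attacking within range, and Attack picks between two fist montages via a semi-random counter, sphere-tracing on notifies to damage and launch the player.
; BPCDamageSystem owns health and drives hit reactions that freeze then resume attacking, plus a delayed ragdoll death that stops AI logic.
; Wrapper functions expose health, damage and movement speed.
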(event `Attack`
  (bind _returnvalue (`self.K2_GetActorLocation`))
  (bind _returnvalue_2 (`self.K2_GetActorLocation`))
  (bind _bpc_damagesystem (`self.BPC_DamageSystem`))
  ;[0.15 0 0 0.5] Attack
  (if (not (`KismetMathLibrary.RandomBool`))
    (set `self.Attack2` (+ 1.0 (`self.Attack2`))))
  (if (>= (`self.Attack2`) 2.0)
    (bind _notifyname (`|PlayMontage` (`self.Mesh`) "/Game/Blueprints/Animation/Enemy/MM_Enemy_Fist_Attack1.MM_Enemy_Fist_Attack1" 1.25)
      (:`then`
        (set `/Game/Blueprints/DamageSystem/BPC_DamageSystem.IsInterruptible` false _bpc_damagesystem :!label _label))
      (:`OnCompleted`
        (set `self.Attack2` 0.0 :!label _label_2)
        (`self.OnAttackEnd` :!label _label_3)
        (set `/Game/Blueprints/DamageSystem/BPC_DamageSystem.IsInterruptible` true _bpc_damagesystem))
      (:`OnInterrupted`
        (goto _label_2))
      (:`OnNotifyBegin`
        (switch `name` _notifyname
          (:`slash`
            (bind _outhit (`KismetSystemLibrary.SphereTraceSingleForObjects` :`Start` _returnvalue :`End` (+ _returnvalue (* (`self.GetActorForwardVector`) (`self.AttackRange`))) :`Radius` 20.0 :`ObjectTypes` (`|MakeArray` "ObjectTypeQuery3" :!type "EObjectTypeQuery Enum") :`DrawTime` 1.0))
            (if true
              (bind (_bblockinghit _binitialoverlap _time _distance _location _impactpoint _normal _impactnormal _physmat _hitactor) (`GameplayStatics.BreakHitResult` _outhit))
              (if (== _hitactor (`GameplayStatics.GetPlayerCharacter` 0))
                (bind _wasdamaged (message `/Game/Blueprints/DamageSystem/BPI_Damagable.TakeDamage` _hitactor (make `/Game/Blueprints/DamageSystem/S_DamageInfo` 30.0 "NewEnumerator1" "NewEnumerator1")))
                (if _wasdamaged
                  (bind _asbf_fps_character (cast `/Game/Blueprints/BF_FPS_Character` _hitactor))
                  (bind (_returnvalue_x _returnvalue_y _returnvalue_z) (`KismetMathLibrary.BreakVector` (* (`KismetMathLibrary.Normal` (- (`self.K2_GetActorLocation` _hitactor) _impactpoint)) 1200.0)))
                  (`self.LaunchCharacter` _asbf_fps_character (`KismetMathLibrary.MakeVector` _returnvalue_x _returnvalue_y (+ _returnvalue_z 250.0)) false false))))))))
    (else
      (bind _notifyname_2 (`|PlayMontage` (`self.Mesh`) "/Game/Blueprints/Animation/Enemy/MM_Enemy_Fist_Attack2.MM_Enemy_Fist_Attack2" 1.25)
        (:`then`
          (goto _label))
        (:`OnCompleted`
          (set `self.Attack2` (+ 1.0 (`self.Attack2`)) :!label _label_4)
          (goto _label_3))
        (:`OnInterrupted`
          (goto _label_4))
        (:`OnNotifyBegin`
          (switch `name` _notifyname_2
            (:`slash`
              (bind _outhit_2 (`KismetSystemLibrary.SphereTraceSingleForObjects` :`Start` _returnvalue_2 :`End` (+ _returnvalue_2 (* (`self.GetActorForwardVector`) (`self.AttackRange`))) :`Radius` 20.0 :`ObjectTypes` (`|MakeArray` "ObjectTypeQuery3" :!type "EObjectTypeQuery Enum") :`DrawTime` 1.0))
              (if true
                (bind (_bblockinghit_2 _binitialoverlap_2 _time_2 _distance_2 _location_2 _impactpoint_2 _normal_2 _impactnormal_2 _physmat_2 _hitactor_2) (`GameplayStatics.BreakHitResult` _outhit_2))
                (if (== _hitactor_2 (`GameplayStatics.GetPlayerCharacter` 0))
                  (bind _wasdamaged_2 (message `/Game/Blueprints/DamageSystem/BPI_Damagable.TakeDamage` _hitactor_2 (make `/Game/Blueprints/DamageSystem/S_DamageInfo` 30.0 "NewEnumerator1" "NewEnumerator6")))
                  (if _wasdamaged_2
                    (bind _asbf_fps_character_2 (cast `/Game/Blueprints/BF_FPS_Character` _hitactor_2))
                    (bind (_returnvalue_x_2 _returnvalue_y_2 _returnvalue_z_2) (`KismetMathLibrary.BreakVector` (* (`KismetMathLibrary.Normal` (- (`self.K2_GetActorLocation` _hitactor_2) _impactnormal_2)) 1200.0)))
                    (`self.LaunchCharacter` _asbf_fps_character_2 (`KismetMathLibrary.MakeVector` _returnvalue_x_2 _returnvalue_y_2 (+ _returnvalue_z_2 250.0)) false false)))))))))))

(event `self.ReceiveBeginPlay`
  (bind _charactermovement (`self.CharacterMovement`))
  ;[0.15 0.1451 0.1004 0.5] Beginplay
  (bind _asaic_enemy_base_aicontroller (cast `/Game/Blueprints/Enemies/EnemyBase/AIC_Enemy_Base_AIController` (`AIBlueprintHelperLibrary.GetAIController` self)))
  (set `self.As AIC Enemy Base AIController` _asaic_enemy_base_aicontroller)
  (set `CharacterMovementComponent.MaxWalkSpeed` 1000.0 _charactermovement)
  (set `CharacterMovementComponent.GroundFriction` 3.0 _charactermovement)
  (set `CharacterMovementComponent.MaxAcceleration` 4048.0 _charactermovement)
  (set `CharacterMovementComponent.BrakingFriction` 0.1 _charactermovement))

(event `Death`
  (bind _mesh (`self.Mesh`))
  ;[0.15 0 0.1211 0.5] Healt
  (`KismetSystemLibrary.Delay` 0.4)
  (`PrimitiveComponent.SetSimulatePhysics` _mesh true)
  (`PrimitiveComponent.SetCollisionEnabled` _mesh "QueryAndPhysics")
  (`BrainComponent.StopLogic` (`AIController.BrainComponent` (`self.As AIC Enemy Base AIController`)) "")
  (`/Game/Blueprints/Enemies/EnemyBase/AIC_Enemy_Base_AIController.SetStateAsDead` (`self.As AIC Enemy Base AIController`))
  (`ActorComponent.K2_DestroyComponent` (`self.CapsuleComponent`)))

(event `self.ReceiveTick`
  (params (DeltaSeconds :type "Float (single-precision)"))
  (bind _returnvalue (`GameplayStatics.GetPlayerPawn` 0))
  (bind _returnvalue_2 (`SceneComponent.K2_GetComponentLocation` (`Actor.RootComponent` _returnvalue)))
  ;[0.04769 0.15 0.002191 0.5] Tick
  (set `self.FocusLocation` _returnvalue_2)
  (if (<= (+ (`KismetMathLibrary.Abs` (.x (- _returnvalue_2 (`self.K2_GetActorLocation` self)))) (`KismetMathLibrary.Abs` (.y (- _returnvalue_2 (`self.K2_GetActorLocation` self))))) 2800.0)
    (`/Game/Blueprints/Enemies/EnemyBase/AIC_Enemy_Base_AIController.SetStateAsAttacking` (`self.As AIC Enemy Base AIController`) _returnvalue false)))

(event `Blocked`
  (params (CanBeParried :type Boolean))
  ;[0.15 0 0.1211 0.5] Healt
  (`KismetSystemLibrary.PrintString` "BLOCKED"))

(event `DamageResponse`
  (params (DamageResponse :type "/Game/Blueprints/DamageSystem/E_DamageResponse Enum" :default "NewEnumerator0"))
  (bind _as_aic_enemy_base_aicontroller (`self.As AIC Enemy Base AIController`))
  (bind _mesh (`self.Mesh`))
  ;[0.15 0 0.1211 0.5] Healt
  (`MovementComponent.StopMovementImmediately` (`self.CharacterMovement`))
  (`/Game/Blueprints/Enemies/EnemyBase/AIC_Enemy_Base_AIController.SetStateAsFrozen` (`self.As AIC Enemy Base AIController`))
  (switch `/Game/Blueprints/DamageSystem/E_DamageResponse` DamageResponse
    (:`NewEnumerator0`
      (`|PlayMontage` _mesh "/Game/Blueprints/Animation/Enemy/MM_HitReact_Left.MM_HitReact_Left" :!label _label_5
        (:`OnCompleted`
          _)
        (:`OnInterrupted`
          _)))
    (:`NewEnumerator1`
      (goto _label_5))
    (:`NewEnumerator6`
      (`|PlayMontage` _mesh "/Game/Blueprints/Animation/Enemy/MM_HitReact_Right.MM_HitReact_Right"
        (:`OnCompleted`
          _)
        (:`OnInterrupted`
          _))))
  (if (`KismetSystemLibrary.IsValid` _as_aic_enemy_base_aicontroller)
    (`/Game/Blueprints/Enemies/EnemyBase/AIC_Enemy_Base_AIController.SetStateAsAttacking` _as_aic_enemy_base_aicontroller (`GameplayStatics.GetPlayerPawn` 0) false)))

(fn `GetCurrentHealt`
  (returns (Healt :type "Float (double-precision)"))
  (return (`/Game/Blueprints/DamageSystem/BPC_DamageSystem.Healt` (`self.BPC_DamageSystem`))))

(fn `GetIdealRange`
  (returns (AttackRadius :type "Float (double-precision)") (DefendRadius :type "Float (double-precision)"))
  (return 0.0 0.0))

(fn `GetMaxHealth`
  (returns (MaxHealt :type "Float (double-precision)"))
  (return (`/Game/Blueprints/DamageSystem/BPC_DamageSystem.MaxHealt` (`self.BPC_DamageSystem`))))

(fn `Heal`
  (params (Amount :type "Float (double-precision)"))
  (returns (NewHealt :type "Float (double-precision)"))
  (bind _newhealt (`/Game/Blueprints/DamageSystem/BPC_DamageSystem.Heal` (`self.BPC_DamageSystem`) Amount))
  (return _newhealt))

(fn `IsDead`
  (returns (IsDead :type Boolean))
  (return (`/Game/Blueprints/DamageSystem/BPC_DamageSystem.IsDead` (`self.BPC_DamageSystem`))))

(fn `SetMovementSpeed`
  (params (Speed :type "/Game/Blueprints/Enemies/EnemyBase/Enums/E_MovementSpeed Enum" :default "NewEnumerator0"))
  (returns (SpeedValue :type "Float (double-precision)"))
  (bind _output_get (set `CharacterMovementComponent.MaxWalkSpeed` (select `/Game/Blueprints/Enemies/EnemyBase/Enums/E_MovementSpeed` Speed :`NewEnumerator1` 200.0 :`NewEnumerator2` 1000.0 :!type "Float (single-precision)") (`self.CharacterMovement`)))
  (return _output_get))

(fn `TakeDamage`
  (params (DamageInfo :type "/Game/Blueprints/DamageSystem/S_DamageInfo Structure"))
  (returns (WasDamaged :type Boolean))
  (bind _wasdamaged (`/Game/Blueprints/DamageSystem/BPC_DamageSystem.TakeDamage` (`self.BPC_DamageSystem`) DamageInfo))
  (return _wasdamaged))

(fn `UserConstructionScript`
  (bind _bpc_damagesystem (`self.BPC_DamageSystem`))
  (bind _bpc_damagesystem_2 (`self.BPC_DamageSystem`))
  (set `/Game/Blueprints/DamageSystem/BPC_DamageSystem.MaxHealt` 30.0 _bpc_damagesystem)
  (set `/Game/Blueprints/DamageSystem/BPC_DamageSystem.Healt` 30.0 _bpc_damagesystem)
  (add `/Game/Blueprints/DamageSystem/BPC_DamageSystem.OnDeath` _bpc_damagesystem_2 (`|CreateDelegate` :!event `Death`))
  (add `/Game/Blueprints/DamageSystem/BPC_DamageSystem.OnBlocked` _bpc_damagesystem_2 (`|CreateDelegate` :!event `Blocked`))
  (add `/Game/Blueprints/DamageSystem/BPC_DamageSystem.OnDamageResponse` _bpc_damagesystem_2 (`|CreateDelegate` :!event `DamageResponse`)))