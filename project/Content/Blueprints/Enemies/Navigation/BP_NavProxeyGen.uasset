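; BP_NavProxeyGen is a nav link proxy that signals enemies to jump when they reach its smart link.
; On SmartLinkReached, it casts the agent to BP_Enemy_Base and writes the link destination to JumpDestination and true to Jump on the AI controller's blackboard.
; The blueprint does not launch the enemy itself; leftover projectile-arc LaunchCharacter experiments remain in the graph but are disconnected.
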(event `self.ReceiveSmartLinkReached`
  (params (Agent :type "Actor Object Reference") (Destination :type "Vector Structure"))
  ; Used for lanching enemys when needto jump
  (bind _asbp_enemy_base (cast `/Game/Blueprints/Enemies/EnemyBase/BP_Enemy_Base` Agent))
  (bind _returnvalue (`AIBlueprintHelperLibrary.GetBlackboard` (`AIBlueprintHelperLibrary.GetAIController` _asbp_enemy_base)))
  (`BlackboardComponent.SetValueAsVector` _returnvalue "JumpDestination" Destination)
  (`BlackboardComponent.SetValueAsBool` _returnvalue "Jump" true)
  (`KismetSystemLibrary.PrintString` (`KismetStringLibrary.Conv_NameToString` "Jump")))