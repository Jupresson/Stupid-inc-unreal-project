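; BP_EnemyBase is an enemy AI base that tracks whether it has seen the player.
; PawnSensing sets a seeing flag for BF_FPS_Character, cleared only when another pawn is seen.
; Tick sets blackboard HasSeenPlayer while seeing, otherwise resets a local memory flag after a delay, never the blackboard key.
; Tick also stores DistanceToTarget as a difference of location vector lengths; an arc-launch snippet is unconnected.
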(event `self.ReceiveTick`
  (params (DeltaSeconds :type "Float (single-precision)"))
  ; Comment
  (`self.GetDistanseOfplayer`)
  (if (`self.SeeingPlayerNow`)
    (set `self.HasSeeingPlayer` true)
    (`self.SetHasSeenPlayer`)
    (elif (`self.HasSeeingPlayer`)
      (`KismetSystemLibrary.Delay` 3.0)
      (set `self.HasSeeingPlayer` false))))

(event `GetDistanseOfplayer`
  ; Comment
  (set `self.DistanceToTarget` (- (`KismetMathLibrary.VSize` (`SceneComponent.K2_GetComponentLocation` (`Actor.RootComponent` (`GameplayStatics.GetPlayerCharacter` 0)))) (`KismetMathLibrary.VSize` (`self.K2_GetActorLocation` self)))))

(event `SetHasSeenPlayer`
  ; Comment
  (`BlackboardComponent.SetValueAsBool` (`AIBlueprintHelperLibrary.GetBlackboard` (`AIBlueprintHelperLibrary.GetAIController` self)) "HasSeenPlayer" true))

(event `self.PawnSensing.OnSeePawn`
  (params (Pawn :type "Pawn Object Reference"))
  ; Comment
  (cast `/Game/Blueprints/BF_FPS_Character` Pawn
    (:`then`
      (set `self.SeeingPlayerNow` true))
    (:`CastFailed`
      (set `self.SeeingPlayerNow` false))))

(fn `UserConstructionScript`)