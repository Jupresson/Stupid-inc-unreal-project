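; Nav link proxy Blueprint that launches enemy AI across gaps or ledges when they need to jump.
; When an agent reaches the smart link, it casts to BP_EnemyAI and computes a custom-arc projectile velocity toward the link destination.
; That velocity is scaled up and applied through LaunchCharacter, overriding the enemy's current movement.
; A disconnected randomized-arc launch variant remains in the graph but never runs.
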(event `self.ReceiveSmartLinkReached`
  (params (Agent :type "Actor Object Reference") (Destination :type "Vector Structure"))
  ; Used for lanching enemys when needto jump
  (bind _asbp_enemy_ai (cast `/Game/Blueprints/BP_EnemyAI` Agent))
  (bind _output_get (set `self.As Character` _asbp_enemy_ai))
  (bind _outlaunchvelocity (`GameplayStatics.SuggestProjectileVelocity_CustomArc` (`Actor.K2_GetActorLocation` _output_get) Destination))
  (`Character.LaunchCharacter` (`self.As Character`) (* _outlaunchvelocity 1.5) true true))