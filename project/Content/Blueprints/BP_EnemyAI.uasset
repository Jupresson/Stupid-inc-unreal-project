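; BP_EnemyAI is an enemy character that chases the player once pawn sensing has seen them.
; Each Tick refreshes the player's position, picks Idle or Move from per-axis distance and a never-cleared seen flag, then runs that state, with Move calling AIMoveTo.
; When the player is near, rotation switches from movement-oriented to controller yaw.
; Jump and Fall states are never selected, and death-screen restart logic is left unconnected.
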(event `GetPlayerPosition`
  ; Getting player position from player reference
  (bind _output_get (set `self.PlayerWorldPosition` (`SceneComponent.K2_GetComponentLocation` (`Actor.RootComponent` (`self.PlayerReference`)))))
  (set `self.PlayerDistance` (`KismetMathLibrary.MakeVector` (`KismetMathLibrary.Abs` (.x (- _output_get (`self.K2_GetActorLocation` self)))) (`KismetMathLibrary.Abs` (.y (- _output_get (`self.K2_GetActorLocation` self)))) (`KismetMathLibrary.Abs` (.z (- _output_get (`self.K2_GetActorLocation` self)))))))

(event `GetPlayerReference`
  ; Getting player reference to variable
  (bind _asbf_fps_character (cast `/Game/Blueprints/BF_FPS_Character` (`GameplayStatics.GetPlayerCharacter` 0)))
  (set `self.PlayerReference` _asbf_fps_character))

(event `self.PawnSensing.OnSeePawn`
  (params (Pawn :type "Pawn Object Reference"))
  ; Seeing player
  (set `self.IsSeeingPlayer` true))

(event `IsPlayerNear`
  (bind (_playerdistance_x _playerdistance_y) (`KismetMathLibrary.BreakVector` (`self.PlayerDistance`)))
  (bind _nearrotationedistance (`self.NearRotationeDistance`))
  ; IsPlayerNear
  (if (<= _playerdistance_x _nearrotationedistance)
    (set `self.NearPlayer` true :!label _label)
    (elif (<= _playerdistance_y _nearrotationedistance)
      (goto _label)
      (else
        (set `self.NearPlayer` false)))))

(event `ChanceRotationSettings`
  (bind _charactermovement (`self.CharacterMovement`))
  ; Fixing rotation settings when player is too near
  (if (`self.NearPlayer`)
    (set `CharacterMovementComponent.bOrientRotationToMovement` false _charactermovement)
    (set `self.bUseControllerRotationYaw` true)
    (else
      (set `CharacterMovementComponent.bOrientRotationToMovement` true _charactermovement)
      (set `self.bUseControllerRotationYaw` false))))

(event `ChooseMovementState`
  (bind (_playerdistance_x _playerdistance_y) (`KismetMathLibrary.BreakVector` (`self.PlayerDistance`)))
  (bind _playerchacedistance (`self.PlayerChaceDistance`))
  ;[0.15 0.02057 0.1495 0.5] ChooseState
  (if (<= _playerdistance_x _playerchacedistance)
    (if (`self.IsSeeingPlayer`) :!label _label_2
      (set `self.CurrentMovementState` "NewEnumerator2")
      (else
        (set `self.CurrentMovementState` "NewEnumerator1")))
    (elif (<= _playerdistance_y _playerchacedistance)
      (goto _label_2)
      (else
        (set `self.CurrentMovementState` "NewEnumerator1")))))

(event `self.ReceiveTick`
  (params (DeltaSeconds :type "Float (single-precision)"))
  ;[0.15 0 0 0.5] Tick
  (`self.GetPlayerReference`)
  (`self.GetPlayerPosition`)
  (`self.IsPlayerNear`)
  (`self.ChanceRotationSettings`)
  (`self.ChooseMovementState`)
  (`self.ApplyMovementState`))

(event `IdleState`)

(event `ApplyMovementState`
  ; ApplyState
  (switch `/Game/Blueprints/E_EnemyAIMovementState` (`self.CurrentMovementState`)
    (:`NewEnumerator1`
      (`self.IdleState`))
    (:`NewEnumerator2`
      (`self.MoveState`))
    (:`NewEnumerator4`
      (`self.JumpState`))
    (:`NewEnumerator9`
      (`self.FallState`))))

(event `MoveState`
  ; MoveState
  (`|AIMoveTo` self (`self.PlayerWorldPosition`) (`self.PlayerReference`)))

(event `JumpState`
  (`self.Jump`))

(event `FallState`)

(fn `UserConstructionScript`)